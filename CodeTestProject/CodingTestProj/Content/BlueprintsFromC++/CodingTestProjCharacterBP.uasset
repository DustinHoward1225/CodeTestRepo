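; Player character Blueprint, apparently over a C++ base, that sets up the player's UI and holds projectile-spawn replication experiments.
; BeginPlay creates the player and sound settings widgets, passing each a reference to the character.
; The SoundMenu input flip-flops mouse cursor and input mode between sound menu and game.
; Three ball-spawn events share one hard-coded SpawnActor; flail, cooldown and projectile hooks are empty, and leftover RPC-style calls are disconnected.
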(event Custom|Spawn%20Ball%20thing
  ;[1 0 0.8386] Replication
  ;;[0 0.4276 1] THIW ONE WORKS
  (Game|SpawnActorfromClass "/Game/BlueprintsFromC++/MyProjectileObjectBP.MyProjectileObjectBP_C" (Math|Transform|MakeTransform "570.000000,-100.000000,450.000000" "0,90.000000, 0" "0.500000,0.500000,0.500000") "Undefined" 0 0))

(event Custom|SpawnBallServer
  ;[1 0 0.8386] Replication
  ;;[0 0.4276 1] THIW ONE WORKS
  (Game|SpawnActorfromClass "/Game/BlueprintsFromC++/MyProjectileObjectBP.MyProjectileObjectBP_C" (Math|Transform|MakeTransform "570.000000,-100.000000,450.000000" "0,90.000000, 0" "0.500000,0.500000,0.500000") "Undefined" 0 0))

(event Custom|Flail%20A%20Server
  ;[1 0 0.8386] Replication
  ;;[0 0.4276 1] THIW ONE WORKS
)

(event Custom|Flail%20Multi
  ;[1 0 0.8386] Replication
  ;;[0 0.4276 1] THIW ONE WORKS
)

(event Custom|SpawnBallMulti
  ;[1 0 0.8386] Replication
  ;;[0 0.4276 1] THIW ONE WORKS
  (Game|SpawnActorfromClass "/Game/BlueprintsFromC++/MyProjectileObjectBP.MyProjectileObjectBP_C" (Math|Transform|MakeTransform "570.000000,-100.000000,450.000000" "0,90.000000, 0" "0.500000,0.500000,0.500000") "Undefined" 0 0))

(event EventBeginPlay
  ;[1 1 1] Adding Widgets to Screen
  (bind _returnvalue (UserInterface|CreateWidget "/Game/BlueprintsFromC++/PlayerWidgetBP.PlayerWidgetBP_C" (Game|GetPlayerController 0)))
  (Variables|/Script/CodingTestProj.PlayerWidget|SetCharacter _returnvalue self)
  (UserInterface|Viewport|AddtoViewport _returnvalue 0)
  (bind _returnvalue_2 (UserInterface|CreateWidget "/Game/Audio/SoundSettingsWidgetBP.SoundSettingsWidgetBP_C" (Game|GetPlayerController 0)))
  (Variables|/Game/Audio/SoundSettingsWidgetBP.SoundSettingsWidgetBP_C|SetChar _returnvalue_2 self)
  (UserInterface|Viewport|AddtoViewport _returnvalue_2 0))

(event Collision|EventActorBeginOverlap
  (params (OtherActor :type Actor%20Object%20Reference)))

(event EventEndOfCooldownBP
  ;[1 1 1] Executes at the end of projectile cooldown
)

(event EventFlailAroundBP
  ;[1 1 1] Executes when the Flail input is entered
)

(event EventSpawnProjectileBP
  ;[1 1 1] Executes when the projectile object itself is spawned
)

(event Input|ActionEvents|InputActionSoundMenu
  (params (Key :type Key%20Structure :default "None"))
  (bind _returnvalue (Game|GetPlayerController 0))
  (bind _returnvalue_2 (Game|GetPlayerController 0))
  ;[1 1 1] Input for switching between Game and Sound settings menu
  (:Pressed
    (Utilities|FlowControl|FlipFlop
      (:A
        (Variables|/Script/Engine.PlayerController|SetbShowMouseCursor _returnvalue_2 true)
        (Input|SetInputModeGameandUI _returnvalue_2 (stale EventBeginPlay _returnvalue_2) "DoNotLock" true))
      (:B
        (Variables|/Script/Engine.PlayerController|SetbShowMouseCursor _returnvalue false)
        (Input|SetInputModeGameOnly _returnvalue)))))

(event Input|ActionEvents|InputActionFlail
  (params (Key :type Key%20Structure :default "None"))
  ;[1 0 0.8386] Replication
  ;;[0 0.4276 1] THIW ONE WORKS
)

(fn ConstructionScript)